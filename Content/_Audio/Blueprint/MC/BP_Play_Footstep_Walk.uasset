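; Animation notify that plays a walking footstep sound matching the surface under the mesh's owning actor.
; When triggered, it line traces on the Visibility channel from the actor's location down along its up vector, with persistent debug drawing.
; The hit's physical surface type selects a stone, wood or water sound, with dirt as the default, played as non-spatialized 2D audio.
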(fn ReceivedNotify
  (params (MeshComp :type Skeletal%20Mesh%20Component%20Object%20Reference) (Animation :type Anim%20Sequence%20Base%20Object%20Reference) (EventReference :type Anim%20Notify%20Event%20Reference%20Structure%20%28by%20ref%29))
  (bind _returnvalue (Components|GetOwner MeshComp))
  (bind _returnvalue_2 (Transformation|GetActorLocation _returnvalue))
  (bind (_outhit _returnvalue_3) (Collision|LineTraceByChannel _returnvalue_2 (+ _returnvalue_2 (* (Transformation|GetActorUpVector _returnvalue) -2e+02)) "TraceTypeQuery1" false 0 "Persistent"))
  (if _returnvalue_3
    (switch Utilities|FlowControl|Switch|SwitchonEPhysicalSurface (Collision|GetSurfaceType _outhit)
      (:SurfaceType_Default
        (Audio|PlaySound2D "/Game/_Audio/MetaSound/Audiosource/MC/Walk/Play_Footstep_Dirt_Walk.Play_Footstep_Dirt_Walk" 1.0 1.0 0.0 0 0))
      (:SurfaceType2
        (Audio|PlaySound2D "/Game/_Audio/MetaSound/Audiosource/MC/Walk/Play_Footstep_Stone_Walk.Play_Footstep_Stone_Walk" 1.0 1.0 0.0 0 0))
      (:SurfaceType3
        (Audio|PlaySound2D "/Game/_Audio/MetaSound/Audiosource/MC/Walk/Play_Footstep_Wood_Walk.Play_Footstep_Wood_Walk" 1.0 1.0 0.0 0 0))
      (:SurfaceType4
        (Audio|PlaySound2D "/Game/_Audio/MetaSound/Audiosource/MC/Walk/Play_Footstep_Water_Walk.Play_Footstep_Water_Walk" 1.0 1.0 0.0 0 0)))
    (return false)))